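; BP_CustomGameMode is a custom game mode that tracks the enemy count and signals a win when none remain.
; On BeginPlay it spawns a BP_UIManager and stores the reference.
; RegisterEnemy and RemoveEnemy raise and lower the count.
; Tick polls that count and calls the UI manager's OnWin on every frame it is zero or below, with no one-shot guard.
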(event `self.ReceiveBeginPlay`
  (bind _returnvalue (`|SpawnActorFromClass` "/Game/BluePrints/Core/BP_UIManager.BP_UIManager_C" (`KismetMathLibrary.MakeTransform` (0.0 0.0 0.0)) "AlwaysSpawn" "MultiplyWithRoot" null null))
  (set `self.UIManagerRef` _returnvalue))

(event `self.ReceiveTick`
  (params (DeltaSeconds :type "Float (single-precision)"))
  (if (<= (`self.NumberOfEnemies`) 0)
    (`/Game/BluePrints/Core/BP_UIManager.OnWin` (`self.UIManagerRef`))))

(event `RegisterEnemy`
  (`/Engine/EditorBlueprintResources/StandardMacros.IncrementInt` (`self.NumberOfEnemies`)))

(event `RemoveEnemy`
  (`/Engine/EditorBlueprintResources/StandardMacros.DecrementInt` (`self.NumberOfEnemies`)))

(fn `UserConstructionScript`)