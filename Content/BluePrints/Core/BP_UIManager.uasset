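; BP_UIManager creates the player's HUD and shows the win and lose screens.
; On BeginPlay it caches the BP_PlayerController and adds a WB_HUD widget to the viewport.
; OnWin and OnLose each reveal their HUD element and pause the game.
; Tick polls the controller's IsDead flag and calls OnLose while it is false, while OnWin has no caller in this graph.
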(event `self.ReceiveBeginPlay`
  (bind _returnvalue (`GameplayStatics.GetPlayerController` 0))
  (`/Engine/EditorBlueprintResources/StandardMacros.IsValid` _returnvalue
    (:`Is Valid`
      (bind _asbp_player_controller (cast `/Game/BluePrints/Core/BP_PlayerController` _returnvalue))
      (bind _output_get (set `self.PlayerControllerRef` _asbp_player_controller))
      (bind _returnvalue_2 (`|CreateWidget` "/Game/Widgets/WB_HUD.WB_HUD_C" _output_get))
      (bind _output_get_2 (set `self.HUD` _returnvalue_2))
      (`UserWidget.AddToViewport` _output_get_2 0))))

(event `self.ReceiveTick`
  (params (DeltaSeconds :type "Float (single-precision)"))
  (if (not (`/Game/BluePrints/Core/BP_PlayerController.IsDead` (`self.PlayerControllerRef`)))
    (`self.OnLose`)))

(event `OnWin`
  (`Widget.SetVisibility` (`/Game/Widgets/WB_HUD.YouWon` (`self.HUD`)) "SelfHitTestInvisible")
  (`GameplayStatics.SetGamePaused` true))

(event `OnLose`
  (`Widget.SetVisibility` (`/Game/Widgets/WB_HUD.YouLose` (`self.HUD`)) "SelfHitTestInvisible")
  (`GameplayStatics.SetGamePaused` true))

(fn `UserConstructionScript`)