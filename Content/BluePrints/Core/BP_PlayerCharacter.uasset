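; BP_PlayerCharacter is the player character Blueprint, carrying weapon components such as an AK47 and a Pistol.
; On BeginPlay it hands each weapon its matching ammo display widget.
; ToggleWeaponVisibility loops over the children of the Weapons component and shows only those whose display name contains the given weapon type's enum name, so visibility depends on component naming.
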(event `self.ReceiveBeginPlay`
  (set `/Game/BluePrints/Actors/Weapons/BP_WeaponBaseComp.AmmoWidget` (`self.AK47_AmmoDisplay`) (`self.AK47`))
  (set `/Game/BluePrints/Actors/Weapons/BP_WeaponBaseComp.AmmoWidget` (`self.Pistol_AmmoDisplay`) (`self.Pistol`)))

(event `ToggleWeaponVisibility`
  (params (WeaponType :type "/Game/BluePrints/Enums/E_WeaponeType Enum" :default "NewEnumerator0"))
  ; Sets the visibility of the weapon based on weapon type
  (for _array_element (`SceneComponent.GetChildrenComponents` (`self.Weapons`) false)
    (`SceneComponent.SetVisibility` _array_element (`KismetStringLibrary.Contains` (`KismetSystemLibrary.GetDisplayName` _array_element) (`|GetEnumeratorNameAsString` WeaponType)) false)))

(fn `UserConstructionScript`)