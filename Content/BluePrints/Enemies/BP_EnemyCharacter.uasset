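; Enemy character Blueprint with health and a kill zone that can end the game when it catches the player.
; Taking damage lowers Health through RemoveHealth, prints the new value, and destroys the actor at zero or below.
; Kill zone overlaps check the BP_AIController for a specific state and its stored player pawn, then print "Game Over" and pause the game.
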(event `self.ReceiveBeginPlay`)

(event `self.ReceiveTick`
  (params (DeltaSeconds :type "Float (single-precision)")))

(event `/Game/BluePrints/Interfaces/BPI_Damageable.TakeDamage`
  (params (Amount :type "Float (double-precision)"))
  (`self.RemoveHealth` Amount)
  (if (<= (`self.Health`) 0.0)
    (`self.K2_DestroyActor`)))

(event `self.KillZone.OnComponentBeginOverlap`
  (params (OverlappedComponent :type "PrimitiveComponent Object Reference") (OtherActor :type "Actor Object Reference") (OtherComp :type "PrimitiveComponent Object Reference") (OtherBodyIndex :type Integer) (bFromSweep :type Boolean) (SweepResult :type "HitResult Structure (by ref)"))
  (bind _returnvalue (`self.GetController`))
  (`/Engine/EditorBlueprintResources/StandardMacros.IsValid` _returnvalue
    (:`Is Valid`
      (bind _asbp_aicontroller (cast `/Game/BluePrints/Enemies/BP_AIController` _returnvalue))
      (if (and (`|EnumEquality` (`/Game/BluePrints/Enemies/BP_AIController.CurrentState` _asbp_aicontroller) "NewEnumerator2") (== (`/Game/BluePrints/Enemies/BP_AIController.PlayerPawnRef` _asbp_aicontroller) OtherActor))
        (`KismetSystemLibrary.PrintString` "Game Over" true true (struct :`R` 1.0 :`B` 0.03047 :`A` 1.0) 30.0)
        (`GameplayStatics.SetGamePaused` true)))))

(fn `RemoveHealth`
  (params (Amount :type "Float (double-precision)"))
  (bind _output_get (set `self.Health` (- (`self.Health`) Amount)))
  (`KismetSystemLibrary.PrintString` (`KismetStringLibrary.Conv_DoubleToString` _output_get) true true (struct :`R` 0.20531 :`G` 1.0 :`A` 1.0) 5.0))

(fn `UserConstructionScript`)