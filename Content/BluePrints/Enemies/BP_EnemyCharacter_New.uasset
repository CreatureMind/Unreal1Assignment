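; Enemy character Blueprint that reacts to damage and ends the game when it catches the player.
; TakeDamage removes health and, if the AI controller is not chasing, switches it to chase; the zero-health check that unpossesses the controller runs only within that branch.
; Overlapping KillZone with the tracked player during chase stops movement and plays an attack montage, then prints Game Over and pauses on completion.
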(event `/Game/BluePrints/Interfaces/BPI_Damageable.TakeDamage`
  (params (Amount :type "Float (double-precision)"))
  (`self.RemoveHealth` Amount)
  ; If it lost healt and he isn't chasing, start chase
  (if (not (`|EnumEquality` (`/Game/BluePrints/Enemies/BP_AIController.CurrentState` (`self.AIControllerRef`)) "NewEnumerator2"))
    (`/Game/BluePrints/Enemies/BP_AIController.UpdateState` (`self.AIControllerRef`) "NewEnumerator2")
    ; if healt reached 0. un possess ai controler
    (if (<= (`self.Health`) 0.0)
      (`Controller.UnPossess` (`self.GetController`)))))

(event `self.KillZone.OnComponentBeginOverlap`
  (params (OverlappedComponent :type "PrimitiveComponent Object Reference") (OtherActor :type "Actor Object Reference") (OtherComp :type "PrimitiveComponent Object Reference") (OtherBodyIndex :type Integer) (bFromSweep :type Boolean) (SweepResult :type "HitResult Structure (by ref)"))
  (bind _aicontrollerref (`self.AIControllerRef`))
  ; Killing the player
  (if (and (`|EnumEquality` (`/Game/BluePrints/Enemies/BP_AIController.CurrentState` _aicontrollerref) "NewEnumerator2") (== (`/Game/BluePrints/Enemies/BP_AIController.PlayerPawnRef` _aicontrollerref) OtherActor))
    (`Controller.StopMovement` (`self.AIControllerRef`))
    (`|PlayMontage` (`self.Mesh`) (`self.AttackMontage`) 2.0
      (:`OnCompleted`
        (`KismetSystemLibrary.PrintString` "Game Over" true true (struct :`R` 1.0 :`B` 0.03047 :`A` 1.0) 30.0)
        (`GameplayStatics.SetGamePaused` true)))))

(fn `UserConstructionScript`
  (`parent.UserConstructionScript`))