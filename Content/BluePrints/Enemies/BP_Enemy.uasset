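; BP_Enemy is an enemy that patrols a looping list of target actors using AI Move To.
; Tick issues the next move whenever the previous one succeeded, advancing the index on success.
; A sphere overlap with the player stops new moves from being issued and prints a debug message, without cancelling the current move.
; A dot-product facing check and a chase move exist only in unconnected, disabled logic.
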(event `self.ReceiveBeginPlay`)

(event `self.ReceiveTick`
  (params (DeltaSeconds :type "Float (single-precision)"))
  (if (`self.IsOverlappingPlayer`)
    (`KismetSystemLibrary.PrintString` "Player in range stoping to patrol")
    (elif (`self.IsSuccessful`)
      (set `self.IsSuccessful` false)
      (`|AIMoveTo` self (`self.GetNextTarget`) null (`self.AcceptanceRadius`)
        (:`OnSuccess`
          (`/Engine/EditorBlueprintResources/StandardMacros.IncrementInt` (`self.CurrentTargetIndex`)
            (:`  `
              (set `self.IsSuccessful` true))))))))

(event `self.Sphere.OnComponentBeginOverlap`
  (params (OverlappedComponent :type "PrimitiveComponent Object Reference") (OtherActor :type "Actor Object Reference") (OtherComp :type "PrimitiveComponent Object Reference") (OtherBodyIndex :type Integer) (bFromSweep :type Boolean) (SweepResult :type "HitResult Structure (by ref)"))
  (set `self.IsOverlappingPlayer` (== OtherActor (`GameplayStatics.GetPlayerPawn` 0))))

(event `self.Sphere.OnComponentEndOverlap`
  (params (OverlappedComponent :type "PrimitiveComponent Object Reference") (OtherActor :type "Actor Object Reference") (OtherComp :type "PrimitiveComponent Object Reference") (OtherBodyIndex :type Integer))
  (set `self.IsOverlappingPlayer` false))

(fn `GetNextTarget`
  (returns (Output :type "Vector Structure"))
  (bind _output_get (set `self.CurrentTargetIndex` (mod (`self.CurrentTargetIndex`) (`KismetArrayLibrary.Array_Length` (`self.TargetsToMoveTo`)))))
  (return (`self.K2_GetActorLocation` (`|GetArrayItem` (`self.TargetsToMoveTo`) _output_get))))

(fn `IsPlayerSeenInRange`
  (params (Range :type "Float (double-precision)"))
  (returns (IsSeen :type Boolean))
  (return (> (`KismetMathLibrary.Dot_VectorVector` (`self.GetActorForwardVector`) (`KismetMathLibrary.Normal` (- (`self.K2_GetActorLocation` (`GameplayStatics.GetPlayerPawn` 0)) (`self.K2_GetActorLocation`)))) Range)))

(fn `UserConstructionScript`)