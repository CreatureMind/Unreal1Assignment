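; Base weapon component that fires physics-driven projectiles, tracks ammo and links an ammo widget to itself.
; Shoot requires ammo and visibility, then spawns a bullet at the first child component, passing damage, coloring it by weapon type and launching it with an impulse.
; It offers ammo refill helpers and finds the left-hand IK child by name.
; An older camera line-trace aiming path remains unconnected.
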(event `self.ReceiveBeginPlay`
  (`KismetSystemLibrary.DelayUntilNextFrame`)
  (`self.SetWidgetParent`))

(event `self.ReceiveTick`
  (params (DeltaSeconds :type "Float (single-precision)"))
  (`self.SetVisibility` (`self.AmmoWidget`) (`self.bVisible`) false))

(event `/Game/BluePrints/Interfaces/BPI_Shootable.Shoot`
  (params (Player :type "/Game/BluePrints/Core/BP_PlayerCharacter Object Reference"))
  (bind _canshoot (`self.CanShoot`))
  (if _canshoot
    (`self.SpawnBullet` (`self.BulletClass`))
    (`self.RemoveAmmo`)
    (`GameplayStatics.PlaySound2D` (`self.GunShotSFX`) 1.0 1.0 0.0 null null)
    (else
      (`KismetSystemLibrary.PrintString` "No bullets!")
      (`GameplayStatics.PlaySound2D` (`self.NoAmmoSFX`) 1.0 1.0 0.0 null null))))

(fn `AddAmmo`
  (params (Amount :type Integer))
  (set `self.CurrentAmmo` (`KismetMathLibrary.Min` (+ Amount (`self.CurrentAmmo`)) (`self.MaxAmmo`)))
  (return))

(fn `ApplyPhysicsAndColor`
  (params (BulletSMA :type "StaticMeshActor Object Reference") (Velocity :type "Vector Structure"))
  (bind _output_get (set `self.BulletRef` (`StaticMeshActor.StaticMeshComponent` BulletSMA)))
  (`self.SetMaterial` _output_get 0 (`BlueprintMapLibrary.Map_Find` (`self.BulletColor`) (`self.WeaponType`)))
  (`self.SetSimulatePhysics` (`self.BulletRef`) true)
  (`self.AddImpulse` (`self.BulletRef`) Velocity "None" false))

(fn `CanShoot`
  (returns (CanShoot :type Boolean))
  (return (and (> (`self.CurrentAmmo`) 0) (`self.bVisible`))))

(fn `GetLeftHandIK`
  (returns (LeftHandIK :type "SceneComponent Object Reference"))
  (locals (LeftHandIKRef :type "SceneComponent Object Reference"))
  (for _array_element (`self.GetChildrenComponents` self false)
    (if (`KismetStringLibrary.EqualEqual_StrStr` (`KismetSystemLibrary.GetObjectName` _array_element) (`self.LeftHandIKName`))
      (return _array_element))))

(fn `IsFullAmmo`
  (returns (IsFull :type Boolean))
  (return (>= (`self.CurrentAmmo`) (`self.MaxAmmo`))))

(fn `RemoveAmmo`
  (bind _result (`/Engine/EditorBlueprintResources/StandardMacros.DecrementInt` (`self.CurrentAmmo`))
    (:`  `
      (set `self.CurrentAmmo` _result))))

(fn `SetWidgetParent`
  (bind _aswb_weapon_ammo (cast `/Game/Widgets/WB_WeaponAmmo` (`WidgetComponent.GetWidget` (`self.AmmoWidget`))))
  (`/Engine/EditorBlueprintResources/StandardMacros.IsValid` _aswb_weapon_ammo
    (:`Is Valid`
      (set `/Game/Widgets/WB_WeaponAmmo.ParentComponent` self _aswb_weapon_ammo))))

(fn `SpawnBullet`
  (params (Bullet :type "/Game/BluePrints/Actors/Weapons/BP_BulletBase Class Reference"))
  (bind _returnvalue (`self.GetChildComponent` self 0))
  (bind _returnvalue_2 (`|SpawnActorFromClass` Bullet (`self.K2_GetComponentToWorld` _returnvalue) "AlwaysSpawn" "MultiplyWithRoot" null (`self.Damage`) null))
  (`self.ApplyPhysicsAndColor` _returnvalue_2 (* (`self.GetForwardVector` _returnvalue) (`self.BulletSpeed`))))