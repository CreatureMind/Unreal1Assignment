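; Base actor for weapon pickups that the player collects by interacting with them.
; On BeginPlay a timeline drives the Weapon component's relative Z, scaled by MaxAmplitude.
; OnInteract adds WeaponType to the player's inventory and destroys the pickup, or prints a message when CanInteract refuses.
; CanInteract refuses only when the player has a current weapon and already holds that type.
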(event `self.ReceiveBeginPlay`
  (bind _returnvalue (`SceneComponent.GetRelativeTransform` (`self.Weapon`)))
  (bind (_direction _float) (`Timeline|Timeline` :!via `PlayFromStart`)
    (:`Update`
      (`SceneComponent.K2_SetRelativeLocation` (`self.Weapon`) (`KismetMathLibrary.MakeVector` (.x (.location _returnvalue)) (.y (.location _returnvalue)) (* _float (`self.MaxAmplitude`))) false false))))

(event `self.ReceiveActorBeginOverlap`
  (params (OtherActor :type "Actor Object Reference")))

(event `/Game/BluePrints/Interfaces/BPI_Interactable.OnInteract`
  (params (InteractingPlayer :type "/Game/BluePrints/Core/BP_PlayerController Object Reference"))
  (bind _isinteractable (`self.CanInteract` InteractingPlayer))
  (if _isinteractable
    (`/Game/BluePrints/Core/BP_PlayerController.AddWeaponToTheInventory` InteractingPlayer (`self.WeaponType`))
    (`self.K2_DestroyActor`)
    (else
      (`KismetSystemLibrary.PrintString` "You already have that weapon."))))

(fn `CanInteract`
  (params (InteractingObject :type "/Game/BluePrints/Core/BP_PlayerController Object Reference"))
  (returns (IsInteractable :type Boolean))
  (`/Engine/EditorBlueprintResources/StandardMacros.IsValid` (`/Game/BluePrints/Core/BP_PlayerController.CurrentWeapon` InteractingObject)
    (:`Is Valid`
      (return (not (`KismetArrayLibrary.Array_Contains` (`/Game/BluePrints/Core/BP_PlayerController.Inventory` InteractingObject) (`self.WeaponType`)))))
    (:`Is Not Valid`
      (return true))))

(fn `UserConstructionScript`)