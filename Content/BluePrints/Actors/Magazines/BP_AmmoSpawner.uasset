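; BP_AmmoSpawner is an actor that scatters random magazines across the ground within its SpawnArea bounds on BeginPlay.
; A loop traces downward from random points in the bounds, drawing persistent debug lines, until TotalToSpawn runs out or MaxAttempts reaches its cap.
; Each hit is raised by HeightFromGround and sphere-checked for crowding.
; Clear spots receive a random class from MagazinesToSpawn.
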(event `self.ReceiveBeginPlay`
  (`self.SpawnRandomMagazine`))

(fn `GetRandomMagazine`
  (returns (Output :type "/Game/BluePrints/Actors/Magazines/BP_PickableMagazineBase Class Reference"))
  (return (`|GetArrayItem` (`self.MagazinesToSpawn`) (`KismetMathLibrary.RandomIntegerInRange` 0 (`KismetArrayLibrary.Array_LastIndex` (`self.MagazinesToSpawn`))))))

(fn `SpawnRandomMagazine`
  (bind (_origin _boxextent) (`KismetSystemLibrary.GetComponentBounds` (`self.SpawnArea`)))
  (bind _returnvalue (`KismetMathLibrary.RandomPointInBoundingBox` _origin _boxextent))
  (while (and (!= (`self.TotalToSpawn`) 0) (< (`self.MaxAttempts`) 100))
    (bind _outhit (`KismetSystemLibrary.LineTraceSingle` :`Start` _returnvalue :`End` (+ _returnvalue (* (`KismetMathLibrary.Vector_Down`) 1000)) :`TraceChannel` "TraceTypeQuery1" :`DrawDebugType` "Persistent"))
    (bind (_bblockinghit _binitialoverlap _time _distance _location) (`GameplayStatics.BreakHitResult` _outhit))
    (if _bblockinghit
      (bind _returnvalue_2 (+ (* (`KismetMathLibrary.Vector_Up`) (`self.HeightFromGround`)) _location))
      (bind _outactors (`KismetSystemLibrary.SphereOverlapActors` _returnvalue_2 50.0 (`|MakeArray` "ObjectTypeQuery1" "ObjectTypeQuery2" :!type "EObjectTypeQuery Enum")))
      (if (<= (`KismetArrayLibrary.Array_Length` _outactors) 1)
        (`|SpawnActorFromClass` (`self.GetRandomMagazine`) (`KismetMathLibrary.MakeTransform` _returnvalue_2) "AdjustIfPossibleButAlwaysSpawn" "MultiplyWithRoot" null null)
        (`/Engine/EditorBlueprintResources/StandardMacros.DecrementInt` (`self.TotalToSpawn`)
          (:`  `
            (`/Engine/EditorBlueprintResources/StandardMacros.IncrementInt` (`self.MaxAttempts`)
              (:`  `
                (`KismetSystemLibrary.PrintString` "Ammo spawned!")))))
        (else
          (`/Engine/EditorBlueprintResources/StandardMacros.IncrementInt` (`self.MaxAttempts`))))
      (else
        (`/Engine/EditorBlueprintResources/StandardMacros.IncrementInt` (`self.MaxAttempts`))))))

(fn `UserConstructionScript`)