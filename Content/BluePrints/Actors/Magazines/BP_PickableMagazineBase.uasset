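; Base actor for magazine pickups that refill a player's compatible weapon with a random ammo amount.
; Interacting requires a valid current weapon and the compatible type in inventory, then adds ammo and destroys the pickup unless that weapon is full.
; A randomly delayed timeline bobs the root vertically and unhides the actor.
; An ammo widget, given a reference to the actor, turns toward the camera every tick.
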(event `self.ReceiveBeginPlay`
  (`parent.ReceiveBeginPlay`)
  (set `self.MainCamera` (`GameplayStatics.GetPlayerCameraManager` 0))
  (`self.StartFloatingAnimation`)
  (`KismetSystemLibrary.DelayUntilNextFrame`)
  (`self.SetWidgetParent`)
  (set `self.CurrentAmmo` (`self.GetAmmoAmount`))
  (`self.SetActorHiddenInGame` true))

(event `self.ReceiveTick`
  (params (DeltaSeconds :type "Float (single-precision)"))
  (`parent.ReceiveTick` DeltaSeconds)
  ; Rotate the text to face the camera all the time
  (`SceneComponent.K2_SetWorldRotation` (`self.AmountText`) (`KismetMathLibrary.FindLookAtRotation` (`SceneComponent.K2_GetComponentLocation` (`self.AmountText`)) (`PlayerCameraManager.GetCameraLocation` (`self.MainCamera`))) false false))

(event `/Game/BluePrints/Interfaces/BPI_Interactable.OnInteract`
  (params (InteractingPlayer :type "/Game/BluePrints/Core/BP_PlayerController Object Reference"))
  (bind _isinteractable (`self.CanInteract` InteractingPlayer))
  (if _isinteractable
    (bind _asbp_weapon_base_comp (`/Game/BluePrints/Core/BP_PlayerController.GetWeaponByType` InteractingPlayer (`self.CompatibleWeapon`)))
    (if (`/Game/BluePrints/Actors/Weapons/BP_WeaponBaseComp.IsFullAmmo` _asbp_weapon_base_comp)
      (`KismetSystemLibrary.PrintString` "The weapons ammo is full.")
      (else
        (`/Game/BluePrints/Actors/Weapons/BP_WeaponBaseComp.AddAmmo` _asbp_weapon_base_comp (`self.CurrentAmmo`))
        (`self.K2_DestroyActor`)))
    (else
      (`KismetSystemLibrary.PrintString` "You don't have the compatiable weapon."))))

(event `StartFloatingAnimation`
  (bind _returnvalue (`SceneComponent.GetRelativeTransform` (`self.DefaultSceneRoot`)))
  (`KismetSystemLibrary.Delay` (`KismetMathLibrary.RandomFloatInRange` 0.0 2.0))
  (`self.SetActorHiddenInGame` false)
  (bind (_direction _float) (`Timeline|Timeline` :!via `PlayFromStart`)
    (:`Update`
      (`SceneComponent.K2_SetRelativeLocation` (`self.DefaultSceneRoot`) (`KismetMathLibrary.MakeVector` (.x (.location _returnvalue)) (.y (.location _returnvalue)) (+ (* _float (`self.MaxAmplitude`)) (`self.FloorOffset`))) false false))))

(fn `CanInteract`
  (params (InteractingObject :type "/Game/BluePrints/Core/BP_PlayerController Object Reference"))
  (returns (IsInteractable :type Boolean))
  (`/Engine/EditorBlueprintResources/StandardMacros.IsValid` (`/Game/BluePrints/Core/BP_PlayerController.CurrentWeapon` InteractingObject)
    (:`Is Valid`
      (return (`KismetArrayLibrary.Array_Contains` (`/Game/BluePrints/Core/BP_PlayerController.Inventory` InteractingObject) (`self.CompatibleWeapon`))))
    (:`Is Not Valid`
      (return false))))

(fn `GetAmmoAmount`
  (returns (Amount :type Integer))
  (return (`KismetMathLibrary.RandomIntegerInRange` (`self.AmmoMin`) (`self.AmmoMax`))))

(fn `SetWidgetParent`
  (bind _aswb_magazine_ammo (cast `/Game/Widgets/WB_MagazineAmmo` (`WidgetComponent.GetWidget` (`self.AmountText`))))
  (`/Engine/EditorBlueprintResources/StandardMacros.IsValid` _aswb_magazine_ammo
    (:`Is Valid`
      (set `/Game/Widgets/WB_MagazineAmmo.ParentActor` self _aswb_magazine_ammo))))

(fn `UserConstructionScript`
  (`parent.UserConstructionScript`))