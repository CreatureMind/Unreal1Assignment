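; Interactable button that moves a referenced wall along its relative X axis and then returns it.
; On interact it waits briefly, plays one timeline forward, then runs a second in reverse, with play rates derived from AnimationSpeed.
; Each update sets X directly from direction, distance and timeline alpha, rather than offsetting the starting position.
; A playing flag blocks retriggering until the return finishes.
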(event `/Game/BluePrints/Interfaces/BPI_Interactable.OnInteract`
  (params (InteractingPlayer :type "/Game/BluePrints/Core/BP_PlayerController Object Reference"))
  (`self.StartMovingAnimation`)
  (`KismetSystemLibrary.PrintString` "Interacted"))

(event `StartMovingAnimation`
  (bind _staticmeshcomponent (`StaticMeshActor.StaticMeshComponent` (`self.WallToMove`)))
  (bind _staticmeshcomponent_2 (`StaticMeshActor.StaticMeshComponent` (`self.WallToMove`)))
  (bind _returnvalue (`SceneComponent.GetRelativeTransform` _staticmeshcomponent))
  (bind _returnvalue_2 (`SceneComponent.GetRelativeTransform` _staticmeshcomponent_2))
  (if (not (`self.IsTimelinePlaying`))
    (set `self.IsTimelinePlaying` true)
    (`KismetSystemLibrary.Delay` 0.2)
    (`TimelineComponent.SetPlayRate` (`self.AnimationTimeline`) (/ 1.0 (* (`self.AnimationSpeed`) 60.0)))
    (bind (_direction _float) (`Timeline|AnimationTimeline` :!via `PlayFromStart`)
      (:`Update`
        (`SceneComponent.K2_SetRelativeLocation` _staticmeshcomponent (`KismetMathLibrary.MakeVector` (`KismetMathLibrary.Conv_IntToDouble` (* (`self.MoveDir`) (* _float (`self.MoveDistance`)))) (.y (.location _returnvalue)) (.z (.location _returnvalue))) false false))
      (:`Finished`
        (`TimelineComponent.SetPlayRate` (`self.Timeline`) (/ 1.0 (* (`self.AnimationSpeed`) 60.0)))
        (bind (_direction_2 _float_2) (`Timeline|Timeline` :!via `ReverseFromEnd`)
          (:`Update`
            (`SceneComponent.K2_SetRelativeLocation` _staticmeshcomponent_2 (`KismetMathLibrary.MakeVector` (`KismetMathLibrary.Conv_IntToDouble` (* (`self.MoveDir`) (* _float_2 (`self.MoveDistance`)))) (.y (.location _returnvalue_2)) (.z (.location _returnvalue_2))) false false))
          (:`Finished`
            (set `self.IsTimelinePlaying` false)))))))

(fn `UserConstructionScript`)